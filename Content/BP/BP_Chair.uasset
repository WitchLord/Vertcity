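; BP_Chair is a possessable chair display that spins slowly until the player walks up to inspect it.
; BeginPlay applies the mesh and material, and Tick adds a fixed per-frame yaw while not in detail mode.
; Overlap by the third-person character stops the spin, shows WBP_PlayerInteraction with UI-only input and cursor, then possesses the chair.
; The Move Right / Left axis rotates its yaw; other axis events are empty.
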(event OnComponentBeginOverlap(Box)
  (params (OverlappedComponent :type Primitive%20Component%20Object%20Reference) (OtherActor :type Actor%20Object%20Reference) (OtherComp :type Primitive%20Component%20Object%20Reference) (OtherBodyIndex :type Integer) (bFromSweep :type Boolean) (SweepResult :type Hit%20Result%20Structure%20%28by%20ref%29))
  (bind _returnvalue (Game|GetPlayerController 0))
  (Utilities|Casting|CastToBP_ThirdPersonCharacter OtherActor)
  (Variables|Default|SetIsInDetail? true)
  (Utilities|FlowControl|Delay 0.2)
  (bind _returnvalue_2 (UserInterface|CreateWidget "/Game/BP/WBP_PlayerInteraction.WBP_PlayerInteraction_C" _returnvalue))
  (UserInterface|Viewport|AddtoPlayerScreen _returnvalue_2)
  (Input|SetInputModeUIOnly _returnvalue _returnvalue_2 "LockOnCapture")
  (Variables|/Script/Engine.PlayerController|SetbShowMouseCursor _returnvalue true)
  (Pawn|Possess (Game|GetPlayerController 0) self))

(event EventBeginPlay
  (bind _chair (Variables|Default|GetChair))
  (Components|StaticMesh|SetStaticMesh _chair (Variables|Default|GetSM_Chair))
  (Rendering|Material|SetMaterial _chair 0 "/Game/ScienceLab/Materials/OfficeProps/MI_Chair.MI_Chair"))

(event EventTick
  (params (DeltaSeconds :type Float%20%28single-precision%29))
  (bind _chair (Variables|Default|GetChair))
  (if (not (Variables|Default|GetIsInDetail?))
    (Transformation|SetRelativeRotation _chair (Math|Rotator|MakeRotator 0.0 0.0 (+ (.yaw (Variables|/Script/Engine.SceneComponent|GetRelativeRotation _chair)) 1.0)) false false)))

(event Input|AxisEvents|InputAxisMoveForward/Backward
  (params (AxisValue :type Float%20%28single-precision%29)))

(event Input|AxisEvents|InputAxisMoveRight/Left
  (params (AxisValue :type Float%20%28single-precision%29))
  (bind _chair (Variables|Default|GetChair))
  (bind _relativerotation (Variables|/Script/Engine.SceneComponent|GetRelativeRotation _chair))
  (Transformation|SetRelativeRotation _chair (Math|Rotator|MakeRotator (.roll _relativerotation) (.pitch _relativerotation) (+ (+ (stale Input|AxisEvents|InputAxisTurnRight/LeftMouse AxisValue) AxisValue) (.yaw _relativerotation))) false false))

(event Input|AxisEvents|InputAxisLookUp/DownMouse
  (params (AxisValue :type Float%20%28single-precision%29)))

(event Input|AxisEvents|InputAxisTurnRight/LeftMouse
  (params (AxisValue :type Float%20%28single-precision%29)))

(fn ConstructionScript)